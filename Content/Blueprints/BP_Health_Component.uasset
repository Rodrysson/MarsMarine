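; Health component Blueprint that tracks current health against a maximum.
; BeginPlay sets current health to the maximum.
; Decrease and add functions clamp the result between zero and the maximum, with only the decrease returning the new value.
; A helper reports whether health is full; nothing here handles death or notifies listeners of changes.
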(event EventBeginPlay
  (Variables|Default|SetCurrentHealth (Variables|Default|GetMaxHealth)))

(fn DecreaseHealth
  (params (Amount :type Float%20%28single-precision%29))
  (bind _output_get (Variables|Default|SetCurrentHealth (Math|Float|Clamp(Float) (- (Variables|Default|GetCurrentHealth) Amount) 0.0 (Variables|Default|GetMaxHealth))))
  (return _output_get))

(fn AddHealth
  (params (HealthToAdd :type Float%20%28single-precision%29))
  (Variables|Default|SetCurrentHealth (Math|Float|Clamp(Float) (+ HealthToAdd (Variables|Default|GetCurrentHealth)) 0.0 (Variables|Default|GetMaxHealth))))

(fn IsHealthFull
  (return (== (Variables|Default|GetCurrentHealth) (Variables|Default|GetMaxHealth))))